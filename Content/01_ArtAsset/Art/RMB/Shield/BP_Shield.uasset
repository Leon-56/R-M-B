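; Energy shield actor that follows BP_Survivor, toggled with F through a timeline that drives appearance, visibility and collision.
; Left-click camera traces that hit the shield add impact points to a capped array, which Tick ages and expires using a wave curve.
; Hits are packed into a one-row canvas render target, position in RGB and curve value in alpha, feeding the dynamic material with hit count and animation time.
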(event Custom|On%20CRT_HitInfo%20Update
  (params (Canvas :type Canvas%20Object%20Reference) (Width :type Integer) (Height :type Integer))
  (CallFunction|UpdateCRTandMaterial Canvas Width Height))

(event Custom|Update%20CRT%20and%20Material
  (params (Canvas :type Canvas%20Object%20Reference) (Width :type Integer) (Height :type Integer))
  ;[1 1 1] 每帧更新CRT和动态材质实例
  (Rendering|ClearRenderTarget2D (Variables|Default|GetCRT_HitInfo) "(R=0.000000,G=0.000000,B=10000.000000,A=100.000000)")
  (for (_array_element _array_index) (Variables|Default|GetHitInfo)
    (Canvas|DrawTexture :self Canvas :ScreenPosition (Math|Vector2D|MakeVector2D (Math|Conversions|ToFloat(Integer) _array_index) 0.0) :ScreenSize "(X=1.000000,Y=1.000000)" :CoordinateSize "(X=1.000000,Y=1.000000)" :RenderColor (Utilities|Struct|MakeLinearColor (.X (Math|Vector4|BreakVector4 _array_element)) (.Y (Math|Vector4|BreakVector4 _array_element)) (.Z (Math|Vector4|BreakVector4 _array_element)) (Math|Curves|GetFloatValue (Variables|Default|GetCurve_WaveTime) (.W (Math|Vector4|BreakVector4 _array_element)))) :BlendMode "BLEND_Opaque" :PivotPoint "(X=0.500000,Y=0.500000)"))
  (bind _returnvalue (Rendering|Material|CreateDynamicMaterialInstance (Variables|Default|GetShield) 0 (Variables|Default|GetMat_Source) "M_Shield_Dynamic" :!class /Script/Engine.PrimitiveComponent))
  (Rendering|Material|SetTextureParameterValue _returnvalue "T_HitInfo" (Variables|Default|GetCRT_HitInfo))
  (Rendering|Material|SetScalarParameterValue _returnvalue "HitNum" (Math|Conversions|ToFloat(Integer) (Utilities|Array|Length (Variables|Default|GetHitInfo))) :!class /Script/Engine.MaterialInstanceDynamic)
  (Rendering|Material|SetScalarParameterValue _returnvalue "AnimTime" (Variables|Default|GetAnimTime) :!class /Script/Engine.MaterialInstanceDynamic))

(event EventBeginPlay
  (bind _returnvalue (Game|GetPlayerController 0))
  (bind _defaultactive (Variables|Default|GetDefaultActive))
  (bind _generateanim (Variables|Default|GetGenerateAnim))
  (Utilities|FlowControl|Sequence
    (:then_0
      (bind _returnvalue_2 (CanvasRenderTarget2D|CreateCanvasRenderTarget2D "/Script/Engine.CanvasRenderTarget2D" (Variables|Default|GetMaxHitNum) 1))
      (bind _output_get (Variables|Default|SetCRT_HitInfo _returnvalue_2))
      (Variables|/Script/Engine.TextureRenderTarget2D|SetAddressX _output_get "TA_Clamp")
      (Variables|/Script/Engine.TextureRenderTarget2D|SetAddressY _output_get "TA_Clamp"))
    (:then_1
      (Input|EnableInput _returnvalue)
      (Variables|/Script/Engine.PlayerController|SetbShowMouseCursor _returnvalue false)
      (EventDispatchers|AssignOnCanvasRenderTargetUpdate (Variables|Default|GetCRT_HitInfo) (delegate Custom|On%20CRT_HitInfo%20Update))
      (Rendering|ClearRenderTarget2D (Variables|Default|GetCRT_HitInfo) "(R=0.000000,G=0.000000,B=10000.000000,A=100.000000)"))
    (:then_2
      (Collision|SetActorEnableCollision _defaultactive)
      (Rendering|SetVisibility (Variables|Default|GetShield) _defaultactive false)
      (bind _output_get_2 (Variables|Default|SetIsActive _defaultactive))
      (if _output_get_2
        (Variables|Default|SetAnimTime 1.0)
        (Components|Timeline|SetNewTime _generateanim (Components|Timeline|GetTimelineLength _generateanim))
        (else
          (Variables|Default|SetAnimTime 0.0)
          (Components|Timeline|SetNewTime _generateanim 0.0))))
    (:then_3
      (bind _returnvalue_3 (Rendering|Material|CreateDynamicMaterialInstance (Variables|Default|GetShield) 0 (Variables|Default|GetMat_Source) "M_Shield_Dynamic" :!class /Script/Engine.PrimitiveComponent))
      (Rendering|Material|SetTextureParameterValue _returnvalue_3 "CRT_HitInfo" (Variables|Default|GetCRT_HitInfo))
      (Rendering|Material|SetScalarParameterValue _returnvalue_3 "HitNum" 0.0 :!class /Script/Engine.MaterialInstanceDynamic))))

(event EventTick
  (params (DeltaSeconds :type Float%20%28single-precision%29))
  (bind _hitinfo (Variables|Default|GetHitInfo))
  ;[1 1 1] 每帧更新碰撞信息数组
  (for (_array_element _array_index) _hitinfo
    (if (< (Math|Curves|GetFloatValue (Variables|Default|GetCurve_WaveTime) (+ (.W (Math|Vector4|BreakVector4 _array_element)) DeltaSeconds)) 0.0)
      (Utilities|Array|RemoveIndex _hitinfo _array_index)
      (else
        (Utilities|Array|SetArrayElem _hitinfo _array_index (Math|Vector4|MakeVector4 (.X (Math|Vector4|BreakVector4 _array_element)) (.Y (Math|Vector4|BreakVector4 _array_element)) (.Z (Math|Vector4|BreakVector4 _array_element)) (+ (.W (Math|Vector4|BreakVector4 _array_element)) DeltaSeconds))))))
  (Class|CanvasRenderTarget2D|UpdateResource (Variables|Default|GetCRT_HitInfo))
  (bind _returnvalue (Actor|GetActorOfClass "/Game/02_Blueprint/03_Survivor/BP_Survivor.BP_Survivor_C"))
  (Transformation|SetActorLocation (Transformation|GetWorldLocation (Variables|/Script/Engine.Character|GetMesh _returnvalue)) false false))

(event Input|MouseEvents|LeftMouseButton
  (params (Key :type Key%20Structure))
  (bind _returnvalue (Game|GetPlayerCameraManager 0))
  (bind _returnvalue_2 (Camera|GetCameraLocation _returnvalue))
  ;[1 1 1] 点击鼠标左键，射线检测成功，则添加碰撞点到数组
  (:Pressed
    (bind (_outhit _returnvalue_3) (Collision|LineTraceByChannel _returnvalue_2 (+ _returnvalue_2 (* (.WorldDirection (Game|Player|ConvertMouseLocationToWorldSpace (Game|GetPlayerController 0))) 1e+04)) "TraceTypeQuery1" false 0 "None" false "(R=1.000000,G=0.000000,B=0.000000,A=0.000000)" "(R=1.000000,G=0.000000,B=0.036963,A=1.000000)"))
    (if (and _returnvalue_3 (Utilities|Enum|Equal(Enum) (Utilities|GetObjectName (.HitActor (Collision|BreakHitResult _outhit))) (Utilities|GetObjectName self)))
      (if (> (Variables|Default|GetMaxHitNum) (Utilities|Array|Length (Variables|Default|GetHitInfo)))
        (Utilities|Array|Add (Variables|Default|GetHitInfo) (Math|Vector4|MakeVector4 (.X (Math|Vector|BreakVector (.Location (Collision|BreakHitResult _outhit)))) (.Y (Math|Vector|BreakVector (.Location (Collision|BreakHitResult _outhit)))) (.Z (Math|Vector|BreakVector (.Location (Collision|BreakHitResult _outhit)))) 0.0))))))

(event Input|KeyboardEvents|F
  (params (Key :type Key%20Structure))
  ;[1 1 1] F键开关护盾
  (:Pressed
    (bind _output_get (Variables|Default|SetIsActive (not (Variables|Default|GetIsActive))))
    (if _output_get
      (Collision|SetActorEnableCollision true)
      (Rendering|SetVisibility (Variables|Default|GetShield) true false)
      (bind _time (Timeline|GenerateAnim Play)
        (:Update
          (Variables|Default|SetAnimTime _time))
        (:Finished
          (if (not (Variables|Default|GetIsActive))
            (Collision|SetActorEnableCollision false)
            (Rendering|SetVisibility (Variables|Default|GetShield) false false))))
      (else
        (Timeline|GenerateAnim Reverse)))))

(fn ConstructionScript
  (Utilities|FlowControl|Sequence
    (:then_0
      (bind _returnvalue (CanvasRenderTarget2D|CreateCanvasRenderTarget2D "/Script/Engine.CanvasRenderTarget2D" (Variables|Default|GetMaxHitNum) 1))
      (bind _output_get (Variables|Default|SetCRT_HitInfo _returnvalue))
      (Variables|/Script/Engine.TextureRenderTarget2D|SetAddressX _output_get "TA_Clamp")
      (Variables|/Script/Engine.TextureRenderTarget2D|SetAddressY _output_get "TA_Clamp"))
    (:then_1
      (Components|StaticMesh|SetStaticMesh (Variables|Default|GetShield) (Variables|Default|GetMesh)))
    (:then_2
      (bind _returnvalue_2 (Rendering|Material|CreateDynamicMaterialInstance (Variables|Default|GetShield) 0 (Variables|Default|GetMat_Source) "M_Shield_Dynamic" :!class /Script/Engine.PrimitiveComponent))
      (Rendering|Material|SetTextureParameterValue _returnvalue_2 "CRT_HitInfo" (Variables|Default|GetCRT_HitInfo))
      (Rendering|Material|SetScalarParameterValue _returnvalue_2 "HitNum" 0.0 :!class /Script/Engine.MaterialInstanceDynamic))))