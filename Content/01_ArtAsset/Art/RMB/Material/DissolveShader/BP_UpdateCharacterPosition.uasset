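; Actor Blueprint that drives the MPC_Dissolve material parameter collection for see-through dissolving when the view of the player character is blocked.
; On BeginPlay it enables the effect and caches the collection's DissolveAmount as the target.
; Each Tick it publishes the player position and line-traces Visibility from camera to character.
; A hit ramps DissolveAmount toward the target over DissolveTime, while no hit ramps it back down, clamped.
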(event EventBeginPlay
  (Rendering|Material|SetScalarParameterValue "/Game/01_ArtAsset/Art/RMB/Material/DissolveShader/MPC_Dissolve.MPC_Dissolve" "EnableDissolve(bool)" 1.0 :!class /Script/Engine.KismetMaterialLibrary)
  (bind _returnvalue (Rendering|Material|GetScalarParameterValue "/Game/01_ArtAsset/Art/RMB/Material/DissolveShader/MPC_Dissolve.MPC_Dissolve" "DissolveAmount(0,1)" :!class /Script/Engine.KismetMaterialLibrary))
  (Variables|Default|SetTarget%20Dissolve%20Amount _returnvalue))

(event EventTick
  (params (DeltaSeconds :type Float%20%28single-precision%29))
  (bind _returnvalue (Game|GetPlayerCharacter 0))
  (bind _returnvalue_2 (Transformation|GetActorLocation _returnvalue))
  (Rendering|Material|SetVectorParameterValue "/Game/01_ArtAsset/Art/RMB/Material/DissolveShader/MPC_Dissolve.MPC_Dissolve" "PlayerPosition" (Math|Conversions|ToLinearColor(Vector) (+ "0, 0, 0" _returnvalue_2)) :!class /Script/Engine.KismetMaterialLibrary)
  (bind _returnvalue_3 (Collision|LineTraceByChannel (Transformation|GetActorLocation (Game|GetPlayerCameraManager 0)) _returnvalue_2 "TraceTypeQuery1" false 0 "None"))
  (if _returnvalue_3
    (Variables|Default|SetSpeed%20Mul 1.0)
    (else
      (Variables|Default|SetSpeed%20Mul -1.0)))
  (Rendering|Material|SetScalarParameterValue "/Game/01_ArtAsset/Art/RMB/Material/DissolveShader/MPC_Dissolve.MPC_Dissolve" "DissolveAmount(0,1)" (Math|Float|Clamp(Float) (+ (* (* (/ (Variables|Default|GetTarget%20Dissolve%20Amount) (Variables|Default|GetDissolve%20Time)) (Variables|Default|GetSpeed%20Mul)) (Utilities|Time|GetWorldDeltaSeconds)) (Variables|Default|GetCurrent%20Dissolve%20Amount)) -0.01 (Variables|Default|GetTarget%20Dissolve%20Amount)) :!class /Script/Engine.KismetMaterialLibrary)
  (bind _output_get (Variables|Default|SetCurrent%20Dissolve%20Amount (Math|Float|Clamp(Float) (+ (* (* (/ (Variables|Default|GetTarget%20Dissolve%20Amount) (Variables|Default|GetDissolve%20Time)) (Variables|Default|GetSpeed%20Mul)) (Utilities|Time|GetWorldDeltaSeconds)) (Variables|Default|GetCurrent%20Dissolve%20Amount)) -0.01 (Variables|Default|GetTarget%20Dissolve%20Amount)))))

(fn ConstructionScript)